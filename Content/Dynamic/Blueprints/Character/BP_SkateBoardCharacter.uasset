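; Skateboarder character that tilts its board to follow the ground under the wheels.
; Each tick, short vertical line traces at the front and back wheel sockets find ground points, falling back to the socket position on a miss.
; The board mesh interpolates toward the look-at rotation between those points, then has its relative yaw locked.
; Getters expose foot IK socket positions and movement input.
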(event `self.ReceiveTick`
  (params (DeltaSeconds :type "Float (single-precision)"))
  (`self.SkateboardIK`))

(fn `GetFootIKPosition`
  (returns (FrontFootIKPosition :type "Vector Structure") (BackFootIKPosition :type "Vector Structure"))
  (bind _sm_skateboard (`self.SM_Skateboard`))
  (`/Engine/EditorBlueprintResources/StandardMacros.IsValid` _sm_skateboard
    (:`Is Valid`
      (return (`SceneComponent.GetSocketLocation` _sm_skateboard "FrontFootIK") (`SceneComponent.GetSocketLocation` _sm_skateboard "BackFootIK")))))

(fn `GetUserMovement`
  (returns (Forward :type "Float (double-precision)") (Right :type "Float (double-precision)"))
  (bind (_movementinput_x _movementinput_y) (`KismetMathLibrary.BreakVector2D` (`self.MovementInput`)))
  (return _movementinput_y _movementinput_x))

(fn `SkateboardIK`
  (bind _sm_skateboard (`self.SM_Skateboard`))
  (bind (_relativerotation_roll _relativerotation_pitch) (`KismetMathLibrary.BreakRotator` (`SceneComponent.RelativeRotation` _sm_skateboard)))
  (bind _hitlocation (`self.WheelTracer` (`SceneComponent.GetSocketLocation` (`self.SM_Skateboard`) "BackWheelIK")))
  (bind _output_get (set `self.BWHitLocation` _hitlocation))
  (bind _hitlocation_2 (`self.WheelTracer` (`SceneComponent.GetSocketLocation` (`self.SM_Skateboard`) "FrontWheelIK")))
  (bind _output_get_2 (set `self.FWHitLocation` _hitlocation_2))
  (bind (_returnvalue_roll _returnvalue_pitch _returnvalue_yaw) (`KismetMathLibrary.BreakRotator` (`KismetMathLibrary.RInterpTo` (`SceneComponent.K2_GetComponentRotation` (`self.SM_Skateboard`)) (`KismetMathLibrary.FindLookAtRotation` _output_get _output_get_2) (`GameplayStatics.GetWorldDeltaSeconds`) 20.0)))
  (`SceneComponent.K2_SetWorldRotation` _sm_skateboard (`KismetMathLibrary.MakeRotator` _returnvalue_roll _returnvalue_pitch _returnvalue_yaw) false false)
  (`SceneComponent.K2_SetRelativeRotation` _sm_skateboard (`KismetMathLibrary.MakeRotator` _relativerotation_roll _relativerotation_pitch 90.0) false false))

(fn `UserConstructionScript`)

(fn `WheelTracer`
  (params (TracePosition :type "Vector Structure"))
  (returns (HitLocation :type "Vector Structure"))
  (bind (_outhit _returnvalue) (`KismetSystemLibrary.LineTraceSingle` (+ TracePosition (0.0 0.0 30.0)) (+ TracePosition (0.0 0.0 -30.0)) "TraceTypeQuery1"))
  (if _returnvalue
    (return (`.Location` (`GameplayStatics.BreakHitResult` _outhit)))
    (else
      (return TracePosition))))